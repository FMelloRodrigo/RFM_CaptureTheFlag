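; Lobby game mode for the main menu that tracks connected and confirmed players and starts the CTF shooter match.
; Interface events update the player lists, then push names and confirmed indexes to every player controller.
; When at least two players are present and the confirmed count matches, it runs a servertravel console command and sends camera fade messages.
; A ServerTraveling flag suppresses login and logout list updates during travel.
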(event `self.K2_PostLogin`
  (params (NewPlayer :type "PlayerController Object Reference"))
  (`parent.K2_PostLogin` NewPlayer)
  (if (not (`self.ServerTraveling`))
    (`self.I_GMMainMenu_PlayerEnter` NewPlayer true)))

(event `self.K2_OnLogout`
  (params (ExitingController :type "Controller Object Reference"))
  (`parent.K2_OnLogout` ExitingController)
  (if (not (`self.ServerTraveling`))
    (bind _asplayer_controller (cast `PlayerController` ExitingController))
    (`self.I_GMMainMenu_PlayerEnter` _asplayer_controller)))

(event `/Game/Blueprints/MainMenu/Interfaces/BPI_GM_MainMenu.I_GMMainMenu_PlayerEnter`
  (params (Controller :type "PlayerController Object Reference") (Update :type Boolean))
  (bind _playerscontrollers (`self.PlayersControllers`))
  (if Update
    (`KismetArrayLibrary.Array_AddUnique` _playerscontrollers Controller)
    (else
      (`KismetArrayLibrary.Array_RemoveItem` _playerscontrollers Controller)))
  (`self.UpdatePlayersNamesArray`)
  (`KismetSystemLibrary.RetriggerableDelay` 0.1) ; TEMP, tentar remover depois
  (`self.DispatchUpdateMessage`))

(event `/Game/Blueprints/MainMenu/Interfaces/BPI_GM_MainMenu.I_GMMainMenu_PlayerConfirm`
  (params (Controller :type "PlayerController Object Reference") (Confirm :type Boolean))
  (bind _playersconfirmed (`self.PlayersConfirmed`))
  (if Confirm
    (`KismetArrayLibrary.Array_AddUnique` _playersconfirmed Controller)
    (else
      (`KismetArrayLibrary.Array_RemoveItem` _playersconfirmed Controller)))
  (`self.UpdateConfirmedPlayersIndexes`)
  (`self.DispatchUpdateMessage`)
  (`self.PlayersReadyCheck`))

(event `PlayersReadyCheck`
  (bind _returnvalue (`KismetArrayLibrary.Array_Length` (`self.PlayersControllers`)))
  (bind _returnvalue_2 (`KismetArrayLibrary.Array_Length` (`self.PlayersConfirmed`)))
  (if (> _returnvalue_2 1)
    (if (and (== _returnvalue_2 _returnvalue) (> _returnvalue 1))
      (`self.ServerTravel` "Lvl_Shooter_CTF"))))

(event `ServerTravel`
  (params (Name :type String))
  (`KismetSystemLibrary.ExecuteConsoleCommand` (`KismetStringLibrary.Concat_StrStr` "servertravel " Name) null)
  (set `self.ServerTraveling` true)
  (for _array_element (`self.PlayersControllers`)
    (message `/Game/Blueprints/MainMenu/Interfaces/BPI_HUD_MainMenu.I_PCMainMenu_CameraFade` _array_element)))

(event `OpenMapDirect`
  (`GameplayStatics.OpenLevelBySoftObjectPtr` "/Game/Maps/Lvl_Shooter_CTF.Lvl_Shooter_CTF"))

(fn `DispatchUpdateMessage`
  (for _array_element (`self.PlayersControllers`)
    (message `/Game/Blueprints/MainMenu/Interfaces/BPI_HUD_MainMenu.I_PCMainMenu_PlayersUpdate` _array_element (`self.PlayersNames`) (`self.PlayerConfirmedIndexes`))))

(fn `I_GMMainMenu_GetPlayers`
  (returns (Controllers :type "Array of PlayerController Object Reference") (Confirmed :type "Array of PlayerController Object Reference"))
  (return (`self.PlayersControllers`) (`self.PlayersConfirmed`)))

(fn `UpdateConfirmedPlayersIndexes`
  (`KismetArrayLibrary.Array_Clear` (`self.PlayerConfirmedIndexes`))
  (for (_array_element _array_index) (`self.PlayersControllers`)
    (`KismetArrayLibrary.Array_Add` (`self.PlayerConfirmedIndexes`) (`KismetMathLibrary.SelectInt` _array_index -1 (`KismetArrayLibrary.Array_Contains` (`self.PlayersConfirmed`) _array_element)))))

(fn `UpdatePlayersNamesArray`
  (`KismetArrayLibrary.Array_Clear` (`self.PlayersNames`))
  (for (_ _array_index) (`self.PlayersControllers`)
    (bind _returnvalue (`GameplayStatics.GetPlayerState` _array_index))
    (`/Engine/EditorBlueprintResources/StandardMacros.IsValid` _returnvalue
      (:`Is Valid`
        (`KismetArrayLibrary.Array_Add` (`self.PlayersNames`) (`PlayerState.GetPlayerName` _returnvalue)))
      (:`Is Not Valid`
        (`KismetSystemLibrary.PrintString` "PLAYER STATE NOT VALID")))))

(fn `UserConstructionScript`)