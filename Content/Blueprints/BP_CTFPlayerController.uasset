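; Player controller for a Capture the Flag mode, holding only temporary team-color debug scaffolding.
; The TEMP event calls UpdateCharacterTeamColor with RedTeam and prints a marker, but only disconnected nodes call it.
; Those unreachable chains also hold a delayed local-server check, a print of the CTF player state's team, and a debug-string flush.
; Possess, Tick and the construction script are empty.
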(event `self.ReceivePossess`
  (params (PossessedPawn :type "Pawn Object Reference")))

(event `TEMP`
  (`self.UpdateCharacterTeamColor` "RedTeam")
  (`KismetSystemLibrary.PrintString` "TEMP"))

(event `self.ReceiveTick`
  (params (DeltaSeconds :type "Float (single-precision)")))

(fn `UserConstructionScript`)