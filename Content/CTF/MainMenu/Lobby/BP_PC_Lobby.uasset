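; Lobby player controller for the CTF main menu that creates the lobby room widget and links it to the game mode.
; Begin play creates the widget directly on remote clients and through a client event on authority.
; Interface messages push player names and confirmation states to the widget, or fade it on the local controller.
; Ready changes route through a server event when remote, then reach the game mode via an interface message.
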(event `self.ReceiveBeginPlay`
  (`/Engine/EditorBlueprintResources/ActorMacros.Switch Has Authority`
    (:`Authority`
      (`self.CLIENT_CreateLobbyHUD`))
    (:`Remote`
      (bind _returnvalue (`|CreateWidget` "/Game/CTF/MainMenu/UI/Lobby/WBP_LobbyRoom_Screen.WBP_LobbyRoom_Screen_C" (`GameplayStatics.GetPlayerController` 0) :!label _label))
      (bind _output_get (set `self.LobbyWidget` _returnvalue))
      (`UserWidget.AddToViewport` _output_get 0))))

(event `CLIENT_CreateLobbyHUD`
  (goto _label))

(event `CLIENT_UpdatePlayersOnLobbyScreen`
  (params (Array :type "Array of String (by ref)") (Confirmed :type "Array of Integer (by ref)"))
  (bind _lobbywidget (`self.LobbyWidget`))
  (`/Engine/EditorBlueprintResources/StandardMacros.IsValid` _lobbywidget
    (:`Is Valid`
      (`/Game/CTF/MainMenu/UI/Lobby/WBP_LobbyRoom_Screen.UpdatePlayersInLobby` _lobbywidget Array Confirmed))))

(event `/Game/CTF/MainMenu/Interfaces/BPI_HUD_MainMenu.I_PCMainMenu_PlayersUpdate`
  (params (Names :type "Array of String (by ref)") (Confirmed :type "Array of Integer (by ref)"))
  (`self.CLIENT_UpdatePlayersOnLobbyScreen` Names Confirmed))

(event `/Game/CTF/MainMenu/Interfaces/BPI_HUD_MainMenu.I_PCMainMenu_ReadyMessage`
  (params (Ready :type Boolean))
  (`/Engine/EditorBlueprintResources/ActorMacros.Switch Has Authority`
    (:`Authority`
      (`self.UpdatePlayerReadyEvent` Ready))
    (:`Remote`
      (`self.SERVER_UpdatePlayerReadyEvent` Ready))))

(event `SERVER_UpdatePlayerReadyEvent`
  (params (Update :type Boolean))
  (`self.UpdatePlayerReadyEvent` Update))

(event `UpdatePlayerReadyEvent`
  (params (Update :type "Boolean (by ref)"))
  (message `/Game/CTF/MainMenu/Interfaces/BPI_GM_MainMenu.I_GMMainMenu_PlayerConfirm` (`GameplayStatics.GetGameMode`) self Update))

(event `/Game/CTF/MainMenu/Interfaces/BPI_HUD_MainMenu.I_PCMainMenu_CameraFade`
  (`self.temp`))

(event `temp`
  (bind _lobbywidget (`self.LobbyWidget`))
  (if (`self.IsLocalController`)
    (`/Engine/EditorBlueprintResources/StandardMacros.IsValid` _lobbywidget
      (:`Is Valid`
        (`/Game/CTF/MainMenu/UI/Lobby/WBP_LobbyRoom_Screen.Fade` _lobbywidget)))))

(fn `UserConstructionScript`)